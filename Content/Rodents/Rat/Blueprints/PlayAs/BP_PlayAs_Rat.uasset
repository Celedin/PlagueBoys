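; Player-controlled rat character that adds sprinting and wall climbing.
; Sprint input switches walk speed between sneak and sprint values.
; Jump launches the rat upward; if a body-arrow trace hits, gravity turns off and the CharacterLaunch timeline keeps pushing it up, with a short timer set for a stop-climb check.
; That check stops the climb when a bottom-arrow trace finds nothing, while releasing Jump or finishing the timeline also restores gravity.
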(event Custom|stop%20climbing
  (bind _bottomarrow (Variables|Default|GetbottomArrow))
  (bind _charactermovement (Variables|Character|GetCharacterMovement))
  (bind _charactermovement_2 (Variables|Character|GetCharacterMovement))
  (bind _returnvalue (Transformation|GetWorldLocation _bottomarrow))
  ;[1 1 1] Rat Climb
  (bind _returnvalue_2 (Collision|LineTraceByChannel _returnvalue (+ _returnvalue (* (Math|Vector|GetForwardVector _bottomarrow) 5e+01)) "TraceTypeQuery1" false 0 "ForDuration"))
  (if (not _returnvalue_2)
    (Utilities|FlowControl|Sequence
      (:then_0
        (Timeline|CharacterLaunch Stop
          (:Update
            (Character|LaunchCharacter "0, 0,250.000000" false true))
          (:Finished
            (Class|MovementComponent|SetPlaneConstraintNormal _charactermovement "0, 0, 0")
            (Variables|/Script/Engine.CharacterMovementComponent|SetGravityScale _charactermovement 1.0)
            (if (Utilities|Time|IsValidTimerHandle (Variables|Default|GetStopCLimbingCustomEventHandle))
              (Utilities|Time|ClearandInvalidateTimerbyHandle (Variables|Default|GetStopCLimbingCustomEventHandle))))))
      (:then_1
        (Class|MovementComponent|SetPlaneConstraintNormal _charactermovement_2 "0, 0, 0")
        (Variables|/Script/Engine.CharacterMovementComponent|SetGravityScale _charactermovement_2 2.0)
        (if (Utilities|Time|IsValidTimerHandle (Variables|Default|GetStopCLimbingCustomEventHandle))
          (Utilities|Time|ClearandInvalidateTimerbyHandle (Variables|Default|GetStopCLimbingCustomEventHandle))
          (Timeline|CharacterLaunch Stop)
          (else
            (Timeline|CharacterLaunch Stop)))))))

(event EventBeginPlay
  ;[1 1 1] Rat Climb
  (Class|MovementComponent|SetPlaneConstraintEnabled (Variables|Character|GetCharacterMovement) true))

(event Input|ActionEvents|InputActionSprint
  (params (Key :type Key%20Structure :default "None"))
  (bind _charactermovement (Variables|Character|GetCharacterMovement))
  ;[1 1 1] Rat Sprint
  (:Pressed
    (Variables|/Script/Engine.CharacterMovementComponent|SetMaxWalkSpeed _charactermovement (Variables|Default|GetRatSprint)))
  (:Released
    (Variables|/Script/Engine.CharacterMovementComponent|SetMaxWalkSpeed _charactermovement (Variables|Default|GetRatSneak))))

(event Input|ActionEvents|InputActionJump
  (params (Key :type Key%20Structure :default "None"))
  (bind _charactermovement (Variables|Character|GetCharacterMovement))
  (bind _charactermovement_2 (Variables|Character|GetCharacterMovement))
  (bind _charactermovement_3 (Variables|Character|GetCharacterMovement))
  (bind _bodyarrow (Variables|Default|GetBodyArrow))
  (bind _returnvalue (Transformation|GetWorldLocation _bodyarrow))
  ;[1 1 1] Rat Climb
  (:Pressed
    (Character|LaunchCharacter "0, 0,1000.000000" false false)
    (bind _returnvalue_2 (Collision|LineTraceByChannel _returnvalue (+ _returnvalue (* (Math|Vector|GetForwardVector _bodyarrow) 5e+01)) "TraceTypeQuery1" false 0 "ForDuration"))
    (if _returnvalue_2
      (Class|MovementComponent|SetPlaneConstraintNormal _charactermovement_2 "0, 0, 0")
      (Variables|/Script/Engine.CharacterMovementComponent|SetGravityScale _charactermovement_2 0.0)
      (bind _returnvalue_3 (Utilities|Time|SetTimerbyFunctionName 0 "stop climbing" 0.04))
      (Timeline|CharacterLaunch PlayFromStart
        (:Update
          (Character|LaunchCharacter "0, 0,250.000000" false true))
        (:Finished
          (Class|MovementComponent|SetPlaneConstraintNormal _charactermovement "0, 0, 0")
          (Variables|/Script/Engine.CharacterMovementComponent|SetGravityScale _charactermovement 1.0)
          (if (Utilities|Time|IsValidTimerHandle (Variables|Default|GetStopCLimbingCustomEventHandle))
            (Utilities|Time|ClearandInvalidateTimerbyHandle (Variables|Default|GetStopCLimbingCustomEventHandle)))))))
  (:Released
    (Class|MovementComponent|SetPlaneConstraintNormal _charactermovement_3 "0, 0, 0")
    (Variables|/Script/Engine.CharacterMovementComponent|SetGravityScale _charactermovement_3 2.0)
    (Timeline|CharacterLaunch Stop)))

(fn ConstructionScript
  (|CallParentFunction))